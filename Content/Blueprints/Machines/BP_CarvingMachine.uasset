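; BP_CarvingMachine is an interactable machine that spawns carved objects of a player-selected type.
; Interacting inside its box switches the player to UI-only input and adds a new WBP_CarvingMachineUI linked back to the machine.
; SelectObject stores the type, and ProduceObject spawns a white BP_CarvedObject of that type at SpawnPoint.
; An OnRep passes selection changes to the MachineUI component's widget, which BeginPlay hides.
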(event Custom|SelectObject
  (params (NewObjectType :type E_ObjectType%20Enum :default "NewEnumerator0"))
  ;[0.15 0.15 0.15 0.5] Oyuncu UI'den bir obje tipine tıklayınca çağrılır.
  (Variables|Default|SetSelectedObjectType NewObjectType))

(event Custom|ProduceObject
  ;[0.15 0.15 0.15 0.5] Produce butonuna basılınca çağrılır.
  (if (not (Variables|Default|GetbIsProducing))
    (Variables|Default|SetbIsProducing true)
    (bind _returnvalue (Game|SpawnActorfromClass "/Game/Blueprints/Object/BP_CarvedObject.BP_CarvedObject_C" (Transformation|GetWorldTransform (Variables|Default|GetSpawnPoint)) "Undefined" "MultiplyWithRoot" 0 0))
    (Variables|/Game/Blueprints/Object/BP_CarvedObject.BP_CarvedObject_C|SetObjectType _returnvalue (Variables|Default|GetSelectedObjectType))
    (Variables|/Game/Blueprints/Object/BP_CarvedObject.BP_CarvedObject_C|SetObjectColor _returnvalue (Class|KismetMathLibrary|LinearColorWhite))
    (Variables|Default|SetbIsProducing false)))

(event EventBeginPlay
  (Widget|SetVisibility (UserInterface|GetUserWidgetObject (Variables|Default|GetMachineUI)) "Hidden"))

(event EventInteract
  (params (Instigator :type Actor%20Object%20Reference) (Interactor :type Character%20Object%20Reference))
  ;[0.15 0.15 0.15 0.5] Oyuncu makineye yaklaşıp E'ye basınca tetiklenir.
  (if (Collision|IsOverlappingActor (Variables|Default|GetInteractionBox) Interactor :!class /Script/Engine.PrimitiveComponent)
    (bind _asplayer_controller (Utilities|Casting|CastToPlayerController (Pawn|GetController Interactor)))
    (Input|SetInputModeUIOnly _asplayer_controller (UserInterface|GetUserWidgetObject (Variables|Default|GetMachineUI)) "DoNotLock" false)
    (Variables|/Script/Engine.PlayerController|SetbShowMouseCursor _asplayer_controller true)
    (bind _returnvalue (UserInterface|CreateWidget "/Game/Blueprints/UI/WBP_CarvingMachineUI.WBP_CarvingMachineUI_C"))
    (UserInterface|Viewport|AddtoViewport _returnvalue 0)
    (Variables|/Game/Blueprints/UI/WBP_CarvingMachineUI.WBP_CarvingMachineUI_C|SetOwningMachine _returnvalue self)))

(fn ConstructionScript)

(fn OnRepSelectedObjectType
  ;[0.15 0.15 0.15 0.5] Bir oyuncu makine UI'sinden obje seçince diğer oyuncuların ekranında da aynı seçimin görünmesini sağlar.
  (bind _aswbp_carving_machine_ui (Utilities|Casting|CastToWBP_CarvingMachineUI (UserInterface|GetUserWidgetObject (Variables|Default|GetMachineUI))))
  (Default|UpdateSelection _aswbp_carving_machine_ui (Variables|Default|GetSelectedObjectType)))

(fn GetInteractText
  (return ""))