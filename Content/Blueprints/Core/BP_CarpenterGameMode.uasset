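; Game mode for a carpenter game that issues random orders (object type, color, reward) and scores deliveries.
; At authoritative BeginPlay it generates an order and sets a one-shot random timer for another.
; GenerateOrder copies the order to BP_CarpenterGameState, updates locally controlled HUDs and spawns an order display actor.
; ProcessDelivery pays full, half (wrong color, tolerance-checked) or zero (wrong type) reward into the budget, then immediately generates another order.
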(event EventBeginPlay
  ;[0.15 0.15 0.15 0.5] Oyun başlayınca ilk siparişi hemen göster, ardından bir sonraki sipariş için timer'ı başlat.
  (if (Ability|HasAuthority)
    (Utilities|FlowControl|Delay 0.5)
    (CallFunction|GenerateOrder)
    (CallFunction|StartOrderTimer)))

(fn ConstructionScript)

(fn GenerateOrder
  ;[0.15 0.15 0.15 0.5] Oyun başlayınca ilk siparişi oluştur.
  (bind _output_get (Variables|Default|SetActiveOrder (Utilities|Struct|MakeS_OrderData (Utilities|Select :Index (Math|Random|RandomIntegerinRange 0 2) :Option%200 "NewEnumerator0" :Option%201 "NewEnumerator1" :Option%202 "NewEnumerator2") (Utilities|Select :Index (Math|Random|RandomIntegerinRange 0 3) :Option%200 "(R=1.000000,G=0.000000,B=0.000000,A=1.000000)" :Option%201 "(R=1.000000,G=1.000000,B=0.000000,A=1.000000)" :Option%202 "(R=0.000000,G=1.000000,B=0.000000,A=1.000000)" :Option%203 "(R=0.000000,G=0.000000,B=1.000000,A=1.000000)") (Math|Random|RandomFloatinRange 5e+01 2e+02))))
  (bind _asbp_carpenter_game_state (Utilities|Casting|CastToBP_CarpenterGameState (Game|GetGameState)))
  (Variables|/Game/Blueprints/Core/BP_CarpenterGameState.BP_CarpenterGameState_C|SetActiveOrder _asbp_carpenter_game_state _output_get)
  (bind _outactors (Actor|GetAllActorsOfClass "/Game/ThirdPerson/Blueprints/BP_ThirdPersonCharacter.BP_ThirdPersonCharacter_C"))
  (for _array_element _outactors
    (if (Pawn|IsLocallyControlled _array_element)
      (Utilities|IsValid (Variables|/Game/ThirdPerson/Blueprints/BP_ThirdPersonCharacter.BP_ThirdPersonCharacter_C|GetHUDOrderWidget _array_element)
        (:Is%20Valid
          (Default|UpdateOrder (Variables|/Game/ThirdPerson/Blueprints/BP_ThirdPersonCharacter.BP_ThirdPersonCharacter_C|GetHUDOrderWidget _array_element) (Variables|/Game/Blueprints/Core/BP_CarpenterGameState.BP_CarpenterGameState_C|GetActiveOrder _asbp_carpenter_game_state))
          (Variables|Default|SetbHasActiveOrder true)
          (bind _asbp_third_person_character (Utilities|Casting|CastToBP_ThirdPersonCharacter (Game|GetPlayerCharacter 0)))
          (Utilities|IsValid (Variables|/Game/ThirdPerson/Blueprints/BP_ThirdPersonCharacter.BP_ThirdPersonCharacter_C|GetHUDWidget _asbp_third_person_character)
            (:Is%20Valid
              (Default|UpdateOrderStatus (Variables|/Game/ThirdPerson/Blueprints/BP_ThirdPersonCharacter.BP_ThirdPersonCharacter_C|GetHUDWidget _asbp_third_person_character) true)
              (Default|CallOnOrderGenerated (Variables|Default|GetActiveOrder))
              (Utilities|IsValid (Variables|Default|GetActiveOrderDisplay)
                (:Is%20Valid
                  (Actor|DestroyActor (Variables|Default|GetActiveOrderDisplay)))
                (:Is%20Not%20Valid
                  _)))
            (:Is%20Not%20Valid
              _))
          (bind _returnvalue (Game|SpawnActorfromClass "/Game/Blueprints/Interactables/BP_OrderDisplay.BP_OrderDisplay_C" (Transformation|GetActorTransform) "Undefined" "MultiplyWithRoot" 0 0))
          (bind _output_get_2 (Variables|Default|SetActiveOrderDisplay _returnvalue))
          (Default|InitOrder _output_get_2 _output_get))))))

(fn StartOrderTimer
  ;[0.15 0.15 0.15 0.5] Sipariş tamamlandıktan sonra rastgele bir süre sonra yeni sipariş üretmek için timer kurar
  ;;[0.15 0.15 0.15 0.5] Belirlenen süre sonunda GenerateOrder'ı otomatik çağırır
  (Utilities|Time|SetTimerbyFunctionName self "GenerateOrder" (Math|Random|RandomFloatinRange (Variables|Default|GetMinOrderInterval) (Variables|Default|GetMaxOrderInterval))))

(fn ProcessDelivery
  (params (DeliveredType :type E_ObjectType%20Enum :default "NewEnumerator0") (DeliveredColor :type Linear%20Color%20Structure))
  (bind _activeorder (Variables|Default|GetActiveOrder))
  (bind (_objecttype _requiredcolor _reward) (Utilities|Struct|BreakS_OrderData _activeorder))
  (bind _returnvalue (- DeliveredColor _requiredcolor))
  (bind (_r _g _b) (Utilities|Struct|BreakLinearColor _returnvalue))
  ;[0.15 0.15 0.15 0.5] Oyuncu siparişi teslim ettiğinde bu fonksiyon çağrılır. Teslim edilen objeyi aktif siparişle karşılaştırır, ödemeyi hesaplar ve bütçeye ekler.
  (if (Variables|Default|GetbHasActiveOrder)
    (if (Utilities|Enum|Equal(Enum) DeliveredType _objecttype)
      (if (<= (Math|Vector|VectorLength (Math|Vector|MakeVector _r _g _b)) 0.1)
        (bind _asbp_carpenter_game_state (Utilities|Casting|CastToBP_CarpenterGameState (Game|GetGameState)))
        (Default|AddBudget _asbp_carpenter_game_state _reward)
        (Variables|Default|SetbHasActiveOrder false)
        (CallFunction|GenerateOrder)
        (else
          (bind _asbp_carpenter_game_state_2 (Utilities|Casting|CastToBP_CarpenterGameState (Game|GetGameState)))
          (Default|AddBudget _asbp_carpenter_game_state_2 (* _reward 0.5))
          (Variables|Default|SetbHasActiveOrder false)
          (CallFunction|GenerateOrder)))
      (else
        (bind _asbp_carpenter_game_state_3 (Utilities|Casting|CastToBP_CarpenterGameState (Game|GetGameState)))
        (Default|AddBudget _asbp_carpenter_game_state_3 0.0)
        (Variables|Default|SetbHasActiveOrder false)
        (CallFunction|GenerateOrder)))))

(fn OnRepActiveOrderDisplay)