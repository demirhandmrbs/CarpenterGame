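; BP_CarpenterGameState is the game state for a carpenter game, holding the replicated budget and active order.
; AddBudget and DeductBudget adjust Budget without authority or balance checks.
; OnRep handlers find the locally controlled BP_ThirdPersonCharacter and push budget and order status to its HUDWidget, and order details to its HUDOrderWidget.
; BeginPlay sets StartingBudget from the authority flag converted to a number, leaving Budget untouched.
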(event EventBeginPlay
  (Variables|Default|SetStartingBudget (Math|Conversions|ToFloat(Boolean) (Ability|HasAuthority))))

(fn ConstructionScript)

(fn OnRepBudget
  ;[0.15 0.15 0.15 0.5] Budget değişince tüm client'larda otomatik tetiklenir.
  (bind _outactors (Actor|GetAllActorsOfClass "/Game/ThirdPerson/Blueprints/BP_ThirdPersonCharacter.BP_ThirdPersonCharacter_C"))
  (for _array_element _outactors
    (if (Pawn|IsLocallyControlled _array_element)
      (Utilities|IsValid (Variables|/Game/ThirdPerson/Blueprints/BP_ThirdPersonCharacter.BP_ThirdPersonCharacter_C|GetHUDWidget _array_element)
        (:Is%20Valid
          (Default|UpdateBudget (Variables|/Game/ThirdPerson/Blueprints/BP_ThirdPersonCharacter.BP_ThirdPersonCharacter_C|GetHUDWidget _array_element) (Variables|Default|GetBudget)))))))

(fn AddBudget
  (params (Amount :type Float%20%28double-precision%29))
  (Variables|Default|SetBudget (+ Amount (Variables|Default|GetBudget))))

(fn DeductBudget
  (params (Amount :type Float%20%28double-precision%29))
  (Variables|Default|SetBudget (- (Variables|Default|GetBudget) Amount)))

(fn OnRepHasActiveOrder
  ;[0.15 0.15 0.15 0.5] HasActiveOrder değişince tüm client'larda tetiklenir.
  (bind _outactors (Actor|GetAllActorsOfClass "/Game/ThirdPerson/Blueprints/BP_ThirdPersonCharacter.BP_ThirdPersonCharacter_C"))
  (for _array_element _outactors
    (if (Pawn|IsLocallyControlled _array_element)
      (Utilities|IsValid (Variables|/Game/ThirdPerson/Blueprints/BP_ThirdPersonCharacter.BP_ThirdPersonCharacter_C|GetHUDWidget _array_element)
        (:Is%20Valid
          (Default|UpdateOrderStatus (Variables|/Game/ThirdPerson/Blueprints/BP_ThirdPersonCharacter.BP_ThirdPersonCharacter_C|GetHUDWidget _array_element) (Variables|Default|GetHasActiveOrder)))))))

(fn OnRepActiveOrder
  (bind _outactors (Actor|GetAllActorsOfClass "/Game/ThirdPerson/Blueprints/BP_ThirdPersonCharacter.BP_ThirdPersonCharacter_C"))
  (for _array_element _outactors
    (if (Pawn|IsLocallyControlled _array_element)
      (Utilities|IsValid (Variables|/Game/ThirdPerson/Blueprints/BP_ThirdPersonCharacter.BP_ThirdPersonCharacter_C|GetHUDOrderWidget _array_element)
        (:Is%20Valid
          (Default|UpdateOrder (Variables|/Game/ThirdPerson/Blueprints/BP_ThirdPersonCharacter.BP_ThirdPersonCharacter_C|GetHUDOrderWidget _array_element) (Variables|Default|GetActiveOrder)))))))