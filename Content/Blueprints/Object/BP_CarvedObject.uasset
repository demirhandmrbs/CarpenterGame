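; BP_CarvedObject is an interactable, colorable object that players pick up, carry and drop.
; Interact routes through the character's ServerPickUp or ServerDrop, depending on whether it is already carried.
; PickUp attaches it to the player at a fixed offset; Drop detaches it and lowers it relative to the carrier's height.
; SetColor sets ObjectColor, whose OnRep applies the color through a dynamic material instance.
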(event Custom|PickUp
  (params (Player :type Character%20Object%20Reference))
  ;[0.15 0.15 0.15 0.5] Oyuncu E tuşuna basınca çağrılır. Objenin taşındığını işaretler ve kimin taşıdığını kaydeder.
  (Variables|Default|SetbIsCarried true)
  (Variables|Default|SetCarryingPlayer Player)
  (Transformation|AttachActorToActor Player "None" "SnapToTarget" "KeepWorld" "KeepWorld" false)
  (Transformation|SetActorRelativeLocation "100.000000,0.000000,50.000000"))

(event Custom|Drop
  (bind _self self)
  (bind _returnvalue (Transformation|GetActorLocation _self))
  (bind (_x _y) (Math|Vector|BreakVector _returnvalue))
  ;[0.15 0.15 0.15 0.5] Taşınan objeyi karakterden ayırır ve dünyaya bırakır.
  (Transformation|DetachFromActor "KeepWorld" "KeepWorld" "KeepWorld")
  (Transformation|SetActorLocation (Math|Vector|MakeVector _x _y (- (.Z (Math|Vector|BreakVector (Transformation|GetActorLocation (Variables|Default|GetCarryingPlayer)))) 9e+01)) false false)
  (Variables|Default|SetbIsCarried false)
  (Variables|Default|SetCarryingPlayer 0))

(event Custom|SetColor
  (params (NewColor :type Linear%20Color%20Structure))
  ;[0.15 0.15 0.15 0.5] Mesh materyalinin sadece objeye özel kopyasını oluşturur ve rengi yeni renk ile değiştirir.
  (Variables|Default|SetObjectColor NewColor))

(event EventInteract
  (params (Instigator :type Actor%20Object%20Reference) (Interactor :type Character%20Object%20Reference))
  (bind _self self)
  ;[0.15 0.15 0.15 0.5] Karakter E tuşuna basınca bu fonksiyon tetiklenir. Obje taşınıyorsa Drop, taşınmıyorsa PickUp çağrılır.
  (if (Variables|Default|GetbIsCarried)
    (bind _asbp_third_person_character (Utilities|Casting|CastToBP_ThirdPersonCharacter Interactor))
    (Default|ServerDrop _asbp_third_person_character _self)
    (else
      (bind _asbp_third_person_character_2 (Utilities|Casting|CastToBP_ThirdPersonCharacter Interactor))
      (Default|ServerPickUp _asbp_third_person_character_2 _self))))

(fn ConstructionScript)

(fn OnRepObjectColor
  (bind _returnvalue (Rendering|Material|CreateDynamicMaterialInstance (Variables|Default|GetObjectMesh) 0 0 "None" :!class /Script/Engine.PrimitiveComponent))
  (Rendering|Material|SetVectorParameterValue _returnvalue "Color" (Variables|Default|GetObjectColor) :!class /Script/Engine.MaterialInstanceDynamic)
  (Rendering|Material|SetMaterial (Variables|Default|GetObjectMesh) 0 _returnvalue))

(fn GetInteractText
  (return ""))